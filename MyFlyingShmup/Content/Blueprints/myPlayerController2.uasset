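; Player controller that tracks score and lives, shows a crosshair mouse cursor, and plays camera shakes at two strengths.
; Score changes are pushed to myGameHUD, while player death removes a life, then either prints Game Over or respawns and notifies the HUD.
; Respawn spawns the game mode's default pawn at a PlayerStart, possesses it and destroys the old pawn.
; A debug O key damages the player pawn.
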(event Custom|ApplyCameraShake
  (Game|Feedback|ClientStartCameraShake "/Game/Blueprints/BP_EnemyDeathCameraShake.BP_EnemyDeathCameraShake_C" 1.0 "CameraLocal" "0, 0, 0"))

(event Custom|ApplyCameraShakePlayer
  (Game|Feedback|ClientStartCameraShake "/Game/Blueprints/BP_EnemyDeathCameraShake.BP_EnemyDeathCameraShake_C" 2.0 "CameraLocal" "0, 0, 0"))

(event Custom|AddToScore
  (params (ValueToAdd :type Float%20%28double-precision%29))
  (bind _output_get (Variables|Default|SetScore (+ ValueToAdd (Variables|Default|GetScore))))
  (bind _asmy_game_hud (Utilities|Casting|CastTomyGameHUD (HUD|GetHUD)))
  (Default|UpdatePlayerScoreUi _asmy_game_hud _output_get))

(event EventBeginPlay
  (Variables|Default|SetbShowMouseCursor true)
  (Variables|Default|SetCurrentMouseCursor "Crosshairs"))

(event EventOnPlayerRespawn
  (bind _returnvalue (Actor|GetActorOfClass "/Script/Engine.PlayerStart"))
  (bind _returnvalue_2 (Game|SpawnActorfromClass (Variables|/Script/Engine.GameModeBase|GetDefaultPawnClass (Game|GetGameMode)) (Transformation|GetActorTransform _returnvalue) "AlwaysSpawn" "MultiplyWithRoot" 0 0))
  (bind _output_get (Variables|Default|SetPreviousPlayerPawn (Game|Player|GetPlayerPawn 0)))
  (Pawn|Possess _returnvalue_2)
  (Actor|DestroyActor _output_get))

(event EventOnPlayerDeath
  (Development|PrintString "Play Player Death Sequence")
  (CallFunction|ModifyPlayerLives -1))

(event EventModifyPlayerLives
  (params (LivesToAdd :type Integer))
  (bind _output_get (Variables|Default|SetCurrentPlayerLives (+ LivesToAdd (Variables|Default|GetCurrentPlayerLives))))
  (if (<= _output_get 0)
    (Development|PrintString "Game Over!")
    (else
      (CallFunction|OnPlayerRespawn)
      (Class|BPIMyFlyingSHMUP|ModifyPlayerLives(Message) (HUD|GetHUD) -1))))

(event Input|KeyboardEvents|DebugKeyO
  (params (Key :type Key%20Structure :default "None") (ActionValue :type Input%20Action%20Value%20Structure))
  (:Pressed
    (Game|Damage|ApplyDamage (Game|Player|GetPlayerPawn 0) 2.5e+02 0 0)))

(fn ConstructionScript)