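; BP_Enemy_B is an enemy that automatically fires BP_EnemyBullet actors in an alternating pattern.
; On BeginPlay it replaces five static mesh material slots with dynamic instances, stores them in DynamicMaterials, and starts a looping one-second timer.
; Each timer tick toggles a FlipFlop whose state selects either a single shot from the main spawn point or a triple shot from all three.
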(event Custom|ShootBullet
  (bind _isa (Utilities|FlowControl|FlipFlop)
    (:A
      _)
    (:B
      _))
  (switch int (Math|Conversions|ToInteger(Boolean) _isa)
    (:0
      (Game|SpawnActorfromClass "/Game/Blueprints/BP_EnemyBullet.BP_EnemyBullet_C" (Transformation|GetWorldTransform (Variables|Default|GetBulletSpawnPoint)) "Undefined" "MultiplyWithRoot" 0 0))
    (:1
      (Game|SpawnActorfromClass "/Game/Blueprints/BP_EnemyBullet.BP_EnemyBullet_C" (Transformation|GetWorldTransform (Variables|Default|GetBulletSpawnPoint2)) "Undefined" "MultiplyWithRoot" 0 0)
      (Game|SpawnActorfromClass "/Game/Blueprints/BP_EnemyBullet.BP_EnemyBullet_C" (Transformation|GetWorldTransform (Variables|Default|GetBulletSpawnPoint3)) "Undefined" "MultiplyWithRoot" 0 0)
      (Game|SpawnActorfromClass "/Game/Blueprints/BP_EnemyBullet.BP_EnemyBullet_C" (Transformation|GetWorldTransform (Variables|Default|GetBulletSpawnPoint)) "Undefined" "MultiplyWithRoot" 0 0))))

(event EventBeginPlay
  (bind _staticmesh (Variables|Default|GetStaticMesh))
  (for _index (range 0 4)
    (bind _returnvalue (Rendering|Material|GetMaterial (Variables|/Script/Engine.StaticMeshComponent|GetStaticMesh _staticmesh) _index))
    (bind _returnvalue_2 (Rendering|Material|CreateDynamicMaterialInstance _staticmesh _index _returnvalue "None" :!class /Script/Engine.PrimitiveComponent))
    (Rendering|Material|SetMaterial _staticmesh _index _returnvalue_2)
    (Utilities|Array|Add (Variables|Default|GetDynamicMaterials) _returnvalue_2))
  (Utilities|Time|SetTimerbyEvent (delegate Custom|ShootBullet) 1.0 true true))

(fn ConstructionScript
  (|CallParentFunction))