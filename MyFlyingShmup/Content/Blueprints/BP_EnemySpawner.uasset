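; Enemy spawner actor that continually spawns BP_Enemy_A at random intervals from BeginPlay onward.
; A timer with a seeded random delay triggers each spawn, then re-queues itself.
; Each spawn samples the StartLocation and EndLocation splines at the same random time, placing the enemy on the first and rotating it to face the matching point on the second.
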(event Custom|SpawnEnemy
  (bind (_startlocation _endlocation) (CallFunction|GetStartandEndLocation))
  (Game|SpawnActorfromClass "/Game/Blueprints/BP_Enemy_A.BP_Enemy_A_C" (Math|Transform|MakeTransform _startlocation (Math|Rotator|FindLookatRotation _startlocation _endlocation) "1.000000,1.000000,1.000000") "Undefined" "MultiplyWithRoot" 0 0)
  (CallFunction|QueueEnemySpawn))

(event Custom|QueueEnemySpawn
  (bind _returnvalue (Utilities|Time|SetTimerbyEvent (delegate Custom|SpawnEnemy) (Math|Random|RandomFloatinRangefromStream (Variables|Default|GetRandomStream) 1.0 5.0) false true))
  (Variables|Default|SetEnemySpawnTimer _returnvalue))

(event EventBeginPlay
  (Class|KismetMathLibrary|ResetRandomStream (Variables|Default|GetRandomStream))
  (CallFunction|QueueEnemySpawn))

(fn ConstructionScript)

(fn GetStartandEndLocation
  (bind _returnvalue (Math|Random|RandomFloatfromStream (Variables|Default|GetRandomStream)))
  (bind _returnvalue_2 (Spline|GetLocationatTime (Variables|Default|GetStartLocation) _returnvalue "World" true))
  (bind _returnvalue_3 (Spline|GetLocationatTime (Variables|Default|GetEndLocation) _returnvalue "World" true))
  (return _returnvalue_2 _returnvalue_3))