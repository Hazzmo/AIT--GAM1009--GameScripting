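; BP_Enemy_C is an enemy turret that aims at the player and fires bullets on a repeating timer.
; BeginPlay starts a looping timer that spawns a BP_EnemyBullet at the BulletSpawn component's transform, always spawning regardless of collision.
; Every tick, it sets TurretBase's world rotation to the yaw of a look-at from the actor to the player pawn, keeping pitch and roll at zero.
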(event Custom|ShootBullet
  (Game|SpawnActorfromClass "/Game/Blueprints/BP_EnemyBullet.BP_EnemyBullet_C" (Transformation|GetWorldTransform (Variables|Default|GetBulletSpawn)) "AlwaysSpawn" "MultiplyWithRoot" 0 0))

(event EventBeginPlay
  (|CallParentFunction)
  (Utilities|Time|SetTimerbyEvent (delegate Custom|ShootBullet) 1.5 true true))

(event EventTick
  (params (DeltaSeconds :type Float%20%28single-precision%29))
  (Transformation|SetWorldRotation (Variables|Default|GetTurretBase) (Math|Rotator|MakeRotator 0.0 0.0 (.yaw (Math|Rotator|FindLookatRotation (Transformation|GetActorLocation) (Transformation|GetActorLocation (Game|Player|GetPlayerPawn 0))))) false false))

(fn ConstructionScript
  (|CallParentFunction))