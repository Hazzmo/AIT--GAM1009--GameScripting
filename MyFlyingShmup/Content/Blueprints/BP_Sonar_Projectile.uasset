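; Sonar pulse actor whose Sphere expands around the player pawn until the actor overlaps something.
; On BeginPlay the Sphere snaps onto the pawn's static mesh, and each Tick moves it to the pawn's location.
; Tick also multiplies its scale by GrowthRate raised to delta seconds, giving frame-rate-independent exponential growth.
; Any actor overlap prints a hit message and destroys the sonar on the next tick.
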(event EventTick
  (params (DeltaSeconds :type Float%20%28single-precision%29))
  (Utilities|FlowControl|Sequence
    (:then_0
      (bind _returnvalue (Utilities|Time|GetWorldDeltaSeconds))
      (Utilities|FlowControl|Sequence
        (:then_0
          (bind _returnvalue_2 (Transformation|GetWorldTransform (Variables|Default|GetSphere))))
        (:then_1
          (bind _returnvalue_3 (Math|Float|Power (Variables|Default|GetGrowthRate) _returnvalue)))))
    (:then_1
      (bind _returnvalue_4 (Game|Player|GetPlayerPawn 0))
      (bind _asbp_my_first_player_pawn (Utilities|Casting|CastToBP_myFirstPlayerPawn _returnvalue_4))
      (bind _returnvalue_5 (Transformation|GetActorLocation _asbp_my_first_player_pawn))
      (Transformation|SetWorldTransform (Variables|Default|GetSphere) (Math|Transform|MakeTransform _returnvalue_5 "0, 0, 0" (* (.scale _returnvalue_2) _returnvalue_3)) false false))))

(event Collision|EventActorBeginOverlap
  (params (OtherActor :type Actor%20Object%20Reference))
  (|CallParentFunction OtherActor)
  (Development|PrintString "SONAR HIT!")
  (Utilities|FlowControl|DelayUntilNextTick)
  (Actor|DestroyActor))

(event EventBeginPlay
  (bind _returnvalue (Game|Player|GetPlayerPawn 0))
  (bind _asbp_my_first_player_pawn (Utilities|Casting|CastToBP_myFirstPlayerPawn _returnvalue))
  (Transformation|AttachComponentToComponent (Variables|Default|GetSphere) (Variables|/Game/Blueprints/BP_myFirstPlayerPawn.BP_myFirstPlayerPawn_C|GetStaticMesh _asbp_my_first_player_pawn) "None" "SnapToTarget" "SnapToTarget" "KeepRelative" true))

(fn ConstructionScript
  (|CallParentFunction))